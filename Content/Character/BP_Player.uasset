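; Player Blueprint that handles weapon firing with single and automatic fire modes.
; AttemtToFire routes single fire through a DoOnce that ResetFire re-arms, while automatic fire bypasses it.
; Both modes share a CanFire gate with a short Delay cooldown.
; Fire is debug-level: it line-traces WorldStatic objects from Sphere1 along the Cube's forward vector, draws the trace and prints the hit actor's name, without applying damage.
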(event `ResetFire`
  (goto _label :!via `Reset`))

(event `self.ReceiveBeginPlay`)

(event `AttemtToFire`
  (switch `/Game/WeaponType` (`self.WeaponType`)
    (:`NewEnumerator0`
      (`/Engine/EditorBlueprintResources/StandardMacros.DoOnce` false :!label _label
        (:`Completed`
          _)))
    (:`NewEnumerator1`
      _))
  (if (`self.CanFire`)
    (set `self.CanFire` false)
    (`self.Fire`)
    (`KismetSystemLibrary.Delay` 0.2)
    (set `self.CanFire` true)))

(fn `Fire`
  (bind _returnvalue (`SceneComponent.K2_GetComponentLocation` (`self.Sphere1`)))
  (`KismetSystemLibrary.PrintString` "Hello")
  (bind _outhit (`KismetSystemLibrary.LineTraceSingleForObjects` :`Start` _returnvalue :`End` (+ (* (`SceneComponent.GetForwardVector` (`self.Cube`)) 1000.0) _returnvalue) :`ObjectTypes` (`|MakeArray` "ObjectTypeQuery1" :!type "EObjectTypeQuery Enum") :`DrawDebugType` "ForOneFrame"))
  (`KismetSystemLibrary.PrintString` (`KismetSystemLibrary.GetDisplayName` (`.HitActor` (`GameplayStatics.BreakHitResult` _outhit)))))

(fn `UserConstructionScript`)